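; BP_NPC is a non-player character that carries random pocket items and reacts to seeing the player.
; On BeginPlay it fills ItemsInPocket with a few random collectible object types.
; AI Perception sight updates drive the Blackboard: sighting sets the player as TargetActor and copies the game mode's NoreityMeter score into Noreity.
; Losing sight clears the target and stores the stimulus location as LastKnownLocation.
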(event `self.ReceiveBeginPlay`
  (for _ (range (+ (`KismetMathLibrary.RandomIntegerInRange` 1 4) 1))
    (`KismetArrayLibrary.Array_Add` (`self.ItemsInPocket`) (cast `/Game/Blueprints/CollectibleObjectType` (`KismetMathLibrary.Conv_IntToByte` (`KismetMathLibrary.RandomIntegerInRange` 0 (enumcount `/Game/Blueprints/CollectibleObjectType`)))))))

(event `self.AIPerception.OnTargetPerceptionUpdated`
  (params (Actor :type "Actor Object Reference") (Stimulus :type "AIStimulus Structure"))
  (`self.HandleSightSense` Actor Stimulus))

(fn `HandleSightSense`
  (params (Actor :type "Actor Object Reference") (Stimulus :type "AIStimulus Structure"))
  (bind (_stimulus_age _stimulus_expirationage _stimulus_strength _stimulus_stimuluslocation _stimulus_receiverlocation _stimulus_tag _stimulus_bsuccessfullysensed) (break `AIStimulus` (`local.Stimulus`)))
  (bind _returnvalue (`AIPerceptionSystem.GetSenseClassForStimulus` Stimulus))
  (if (== _returnvalue "/Script/AIModule.AISense_Sight")
    (if (`self.ActorHasTag` Actor "Player")
      (`BlackboardComponent.SetValueAsObject` (`AIBlueprintHelperLibrary.GetBlackboard` null) "TargetActor" (`KismetMathLibrary.SelectObject` (`GameplayStatics.GetPlayerCharacter` 0) null _stimulus_bsuccessfullysensed))
      (if _stimulus_bsuccessfullysensed
        (bind _asbp_third_person_game_mode (cast `/Game/Blueprints/BP_ThirdPersonGameMode` (`GameplayStatics.GetGameMode`)))
        (`BlackboardComponent.SetValueAsFloat` (`AIBlueprintHelperLibrary.GetBlackboard` null) "Noreity" (`/Game/Blueprints/NoreityMeter.NoreityScore` (`/Game/Blueprints/BP_ThirdPersonGameMode.NoreityMeter` _asbp_third_person_game_mode)))
        (else
          (`BlackboardComponent.SetValueAsVector` (`AIBlueprintHelperLibrary.GetBlackboard` null) "LastKnownLocation" _stimulus_stimuluslocation)))
      (else
        (return)))
    (else
      (return))))

(fn `UserConstructionScript`)