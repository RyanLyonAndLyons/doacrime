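; Holder actor for a baby that, judging by its name, is unloaded through candy spamming; only the drop step is implemented here.
; DropTheBaby teleports the held Baby to SpawnPoint, enables mesh physics and plays its giggle.
; It also attaches an InteractingTrigger child actor component to the baby at runtime, then clears the reference.
; Event graph is empty, so the drop relies on an external call.
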(fn `DropTheBaby`
  (bind _baby (`self.Baby`))
  (`/Engine/EditorBlueprintResources/StandardMacros.IsValid` (`self.Baby`)
    (:`Is Valid`
      (`self.K2_SetActorTransform` _baby (`SceneComponent.K2_GetComponentToWorld` (`self.SpawnPoint`)) false false)
      (`PrimitiveComponent.SetSimulatePhysics` (`StaticMeshActor.StaticMeshComponent` _baby) true)
      (bind _returnvalue (`AddComponent|NODE_AddChildActorComponent-0` :`self` _baby))
      (`ChildActorComponent.SetChildActorClass` _returnvalue "/Game/Blueprints/InteractingTrigger_Blueprint.InteractingTrigger_Blueprint_C")
      (`/Game/Blueprints/BP_Baby.BabyGiggle` _baby)
      (set `self.Baby` null))))

(fn `UserConstructionScript`
  (`parent.UserConstructionScript`))