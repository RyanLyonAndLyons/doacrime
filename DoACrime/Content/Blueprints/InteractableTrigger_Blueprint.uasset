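; InteractableTrigger is a trigger actor that registers its parent actor as the player character's current interactable while the player overlaps it.
; On begin overlap it also auto-collects a grounded CollectibleObject parent tagged as a pickup.
; On end overlap it clears the interactable, and an NPC-tagged parent uncrouches and walks to a new point after a random delay.
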(event `self.ReceiveBeginPlay`
  (set `self.Interactable` (`self.GetParentActor`)))

(event `self.ReceiveActorBeginOverlap`
  (params (OtherActor :type "Actor Object Reference"))
  (bind _returnvalue (`self.GetParentActor`))
  (if (`self.ActorHasTag` OtherActor "Player")
    (cast `/Game/Blueprints/BP_ThirdPersonGameMode` (`GameplayStatics.GetGameMode`)
      (:`then`
        (bind _asbp_third_person_character (cast `/Game/Blueprints/BP_ThirdPersonCharacter` (`GameplayStatics.GetPlayerCharacter` 0))
          (:`then`
            (set `/Game/Blueprints/BP_ThirdPersonCharacter.CurrentInteractable` (`self.Interactable`) _asbp_third_person_character)
            (if (`self.ActorHasTag` _returnvalue "PickUpObject")
              (bind _ascollectible_object_blueprint (cast `/Game/Blueprints/CollectibleObject_Blueprint` _returnvalue))
              (if (`/Game/Blueprints/CollectibleObject_Blueprint.IsGrounded` _ascollectible_object_blueprint)
                (`/Game/Blueprints/CollectibleObject_Blueprint.Collect Object` _ascollectible_object_blueprint))))
          (:`CastFailed`
            (`KismetSystemLibrary.PrintString` "Failed Cast to Player"))))
      (:`CastFailed`
        (`KismetSystemLibrary.PrintString` "Failed Cast for Game Mode")))))

(event `self.ReceiveActorEndOverlap`
  (params (OtherActor :type "Actor Object Reference"))
  (if (`self.ActorHasTag` OtherActor "Player")
    (cast `/Game/Blueprints/BP_ThirdPersonGameMode` (`GameplayStatics.GetGameMode`))
    (bind _asbp_third_person_character (cast `/Game/Blueprints/BP_ThirdPersonCharacter` (`GameplayStatics.GetPlayerCharacter` 0)))
    (set `/Game/Blueprints/BP_ThirdPersonCharacter.CurrentInteractable` null _asbp_third_person_character)
    (if (`self.ActorHasTag` (`self.GetParentActor`) "NPC")
      (`KismetSystemLibrary.Delay` (`KismetMathLibrary.RandomFloatInRange` 1.0 5.0))
      (bind _asbp_npc (cast `/Game/Blueprints/BP_NPC` (`self.GetParentActor`)))
      (`Character.UnCrouch` _asbp_npc)
      (`/Game/Blueprints/BP_NPC.WalkToNewPoint_Event` _asbp_npc))))

(fn `UserConstructionScript`)