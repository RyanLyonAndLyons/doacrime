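; SpamToUnload actor that wobbles its static mesh with a rummaging sound when StartShake is called.
; StartShake saves the mesh transform, resets a counter and sets the Shaking flag.
; Tick then uses a short Delay to alternate small opposite rotations for a few steps, then holds the saved rotation.
; Shaking is never cleared here, and the un-reset DoOnce plays the sound only on the first shake.
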(event `self.ReceiveTick`
  (params (DeltaSeconds :type "Float (single-precision)"))
  (bind _shakingcounter (`self.ShakingCounter`))
  (bind _staticmeshcomponent (`self.StaticMeshComponent`))
  (bind _returnvalue (`SceneComponent.K2_GetComponentToWorld` _staticmeshcomponent))
  (if (`self.Shaking`)
    (`|ExecutionSequence`
      (:`then_0`
        (`/Engine/EditorBlueprintResources/StandardMacros.DoOnce` false
          (:`Completed`
            (`GameplayStatics.PlaySoundAtLocation` "/Game/Audio/SQ_Rummage.SQ_Rummage" (`SceneComponent.K2_GetComponentLocation` (`self.StaticMeshComponent`)) (struct) 1.0 1.0 0.0 null null null null))))
      (:`then_1`
        (`KismetSystemLibrary.Delay` 0.05)
        (bind _output_get (set `self.ShakingCounter` (+ _shakingcounter 1)))
        (if (<= _shakingcounter 9)
          (if (`KismetMathLibrary.Conv_IntToBool` (mod _output_get 2))
            (`SceneComponent.K2_SetWorldRotation` _staticmeshcomponent (`KismetMathLibrary.TransformRotation` _returnvalue (struct :`Pitch` -1.0 :`Roll` -1.0)) false false)
            (else
              (`SceneComponent.K2_SetWorldRotation` _staticmeshcomponent (`KismetMathLibrary.TransformRotation` _returnvalue (struct :`Pitch` 1.0 :`Roll` 1.0)) false false)))
          (else
            (`SceneComponent.K2_SetWorldRotation` _staticmeshcomponent (`KismetMathLibrary.TransformRotation` (`self.ObjectOriginalTransform`)) false false)))))))

(fn `StartShake`
  (set `self.ObjectOriginalTransform` (`SceneComponent.K2_GetComponentToWorld` (`self.StaticMeshComponent`)))
  (set `self.ShakingCounter` 0)
  (set `self.Shaking` true))

(fn `UserConstructionScript`)