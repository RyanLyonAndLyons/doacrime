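; GoalTrigger_Blueprint is a goal trigger that detects when an actor tagged "Ball" overlaps it.
; On that overlap it casts the game mode to BP_ThirdPersonGameMode, updates a task on its TaskListWidget, and spawns the NS_Confetti effect at the trigger's location.
; An older activate, delay and deactivate chain for an NSConfetti component remains in the graph but is never executed.
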(event `self.ReceiveActorBeginOverlap`
  (params (OtherActor :type "Actor Object Reference"))
  (if (`self.ActorHasTag` OtherActor "Ball")
    (bind _asbp_third_person_game_mode (cast `/Game/Blueprints/BP_ThirdPersonGameMode` (`GameplayStatics.GetGameMode`)))
    (`/Game/Blueprints/TaskListWidget.UpdateTask` (`/Game/Blueprints/BP_ThirdPersonGameMode.TaskListWidget` _asbp_third_person_game_mode) "NewEnumerator3")
    (`NiagaraFunctionLibrary.SpawnSystemAtLocation` "/Game/VFX/NS_Confetti.NS_Confetti" (`self.K2_GetActorLocation`))))

(fn `UserConstructionScript`)