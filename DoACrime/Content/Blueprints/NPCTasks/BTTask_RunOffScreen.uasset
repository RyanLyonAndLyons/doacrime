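; Behavior tree task that makes an NPC run off the map and removes it from the game.
; On AI execute, it triples the BP_NPC's max walk speed and uses AIMoveTo toward the OffMap actor held by BP_ThirdPersonGameMode.
; The NPC is destroyed whether the move succeeds or fails, and the task finishes with the matching result.
; A failed cast stops the graph without finishing the task.
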(event `self.ReceiveExecuteAI`
  (params (OwnerController :type "AIController Object Reference") (ControlledPawn :type "Pawn Object Reference"))
  (bind _asbp_npc (cast `/Game/Blueprints/BP_NPC` ControlledPawn))
  (bind _charactermovement (`Character.CharacterMovement` _asbp_npc))
  (set `CharacterMovementComponent.MaxWalkSpeed` (* (`CharacterMovementComponent.MaxWalkSpeed` _charactermovement) 3.0) _charactermovement)
  (bind _asbp_third_person_game_mode (cast `/Game/Blueprints/BP_ThirdPersonGameMode` (`GameplayStatics.GetGameMode`)))
  (`|AIMoveTo` ControlledPawn (0.0 0.0 0.0) (`/Game/Blueprints/BP_ThirdPersonGameMode.OffMap` _asbp_third_person_game_mode)
    (:`OnSuccess`
      (`Actor.K2_DestroyActor` _asbp_npc)
      (`self.FinishExecute` true))
    (:`OnFail`
      (`Actor.K2_DestroyActor` _asbp_npc)
      (`self.FinishExecute` false))))