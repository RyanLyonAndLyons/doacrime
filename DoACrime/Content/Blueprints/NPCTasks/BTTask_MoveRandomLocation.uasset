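; Behavior Tree task that sends a BP_NPC wandering to a random reachable point around its current location.
; It first sets the NPC's state to the first enum entry and mirrors it to the NPCState Blackboard key.
; An AI Move To then drives the pawn within a configurable radius and acceptance radius, finishing the task as success or failure based on the move result.
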(event `self.ReceiveExecuteAI`
  (params (OwnerController :type "AIController Object Reference") (ControlledPawn :type "Pawn Object Reference"))
  (bind _asbp_npc (cast `/Game/Blueprints/BP_NPC` ControlledPawn))
  (bind _output_get (set `/Game/Blueprints/BP_NPC.CurrentNPCState` "NewEnumerator0" _asbp_npc))
  (`BTFunctionLibrary.SetBlackboardValueAsEnum` (make `BlackboardKeySelector` :`SelectedKeyName` "NPCState") _output_get)
  (`|AIMoveTo` ControlledPawn (`NavigationSystemV1.K2_GetRandomReachablePointInRadius` (`Actor.K2_GetActorLocation` ControlledPawn) (`self.Radius`) null null) null (`self.Acceptance Radius`)
    (:`OnSuccess`
      (`self.FinishExecute` true))
    (:`OnFail`
      (`self.FinishExecute` false))))