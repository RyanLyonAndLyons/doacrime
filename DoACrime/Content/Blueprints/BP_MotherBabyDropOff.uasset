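; BP_MotherBabyDropOff is a drop-off trigger, hosted as a child actor of BP_Mother_Blueprint, that hands a baby over to that mother.
; It accepts an overlapping baby or takes one held by the player, then disables its physics and snaps it to the mother's SpawnBabyPoint.
; The mother plays a walk animation and AI-moves to a random game mode OffMap point.
; On success or failure, both vanish in a poof effect.
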(event `self.ReceiveBeginPlay`
  (bind _asbp_mother_blueprint (cast `/Game/Blueprints/BP_Mother_Blueprint` (`self.GetParentActor`)))
  (set `self.Mother` _asbp_mother_blueprint))

(event `self.ReceiveActorBeginOverlap`
  (params (OtherActor :type "Actor Object Reference"))
  (bind _mother (`self.Mother`))
  (bind _mother_2 (`self.Mother`))
  (bind _spawnbabypoint (`/Game/Blueprints/BP_Mother_Blueprint.SpawnBabyPoint` (`self.Mother`)))
  (if (`self.ActorHasTag` OtherActor "Baby")
    (bind _asbp_baby (cast `/Game/Blueprints/BP_Baby` OtherActor))
    (bind _output_get (set `self.Baby` _asbp_baby))
    (`PrimitiveComponent.SetSimulatePhysics` (`StaticMeshActor.StaticMeshComponent` (`self.Baby`)) false :!label _label)
    (`self.K2_SetActorTransform` _output_get (`SceneComponent.K2_GetComponentToWorld` _spawnbabypoint) false false)
    (`self.K2_AttachToComponent` (`self.Baby`) _spawnbabypoint "None" "SnapToTarget" "SnapToTarget" "SnapToTarget" false)
    (`SkeletalMeshComponent.PlayAnimation` (`Character.Mesh` _mother) "/Game/Characters/Mannequins/Animations/Manny/MM_Walk_Fwd.MM_Walk_Fwd" true)
    (bind _asbp_third_person_game_mode (cast `/Game/Blueprints/BP_ThirdPersonGameMode` (`GameplayStatics.GetGameMode`)))
    (`|AIMoveTo` _mother (`PawnMovementComponent.GetPawnOwner` (`Character.CharacterMovement` (`self.Mother`))) (`self.K2_GetActorLocation` (`KismetArrayLibrary.Array_Random` (`/Game/Blueprints/BP_ThirdPersonGameMode.OffMap` _asbp_third_person_game_mode))) null 100.0
      (:`OnSuccess`
        _)
      (:`OnFail`
        _))
    (`NiagaraFunctionLibrary.SpawnSystemAtLocation` "/Game/VFX/NS_Poof.NS_Poof" (`self.K2_GetActorLocation` _mother_2) (struct) (2.0 2.0 2.0))
    (`self.K2_DestroyActor` (`self.Baby`))
    (`self.K2_DestroyActor` _mother_2)
    (elif (`self.ActorHasTag` OtherActor "Player")
      (bind _asbp_third_person_character (cast `/Game/Blueprints/BP_ThirdPersonCharacter` OtherActor))
      (bind _asbp_baby_2 (cast `/Game/Blueprints/BP_Baby` (`/Game/Blueprints/BP_ThirdPersonCharacter.HeldObject` _asbp_third_person_character)))
      (set `self.Baby` _asbp_baby_2)
      (`/Game/Blueprints/BP_ThirdPersonCharacter.DropHeldObject` _asbp_third_person_character)
      (goto _label))))

(fn `UserConstructionScript`)