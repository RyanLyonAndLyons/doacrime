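; AI controller for BP_NPC that reacts to perceived threats by scaring the NPC.
; Perception updates feed HandleSenses: seeing a notorious player or hearing gun or notorious chitter sounds sets a scared state, stopping movement on sight or state change.
; Custom events handle idling, random wandering and fleeing, which also doubles the player's walk speed.
; Behavior tree startup and those events' bindings are disconnected.
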(event `self.ReceiveBeginPlay`)

(event `self.ReceivePossess`
  (params (PossessedPawn :type "Pawn Object Reference"))
  (bind _asbp_npc (cast `/Game/Blueprints/BP_NPC` PossessedPawn))
  (set `self.NPC` _asbp_npc))

(event `AvoidPlayer_Event`
  (bind _returnvalue (`self.K2_GetActorLocation`))
  (bind _asbp_third_person_character (cast `/Game/Blueprints/BP_ThirdPersonCharacter` (`GameplayStatics.GetPlayerCharacter` 0)))
  (bind _charactermovement (`Character.CharacterMovement` _asbp_third_person_character))
  (set `CharacterMovementComponent.MaxWalkSpeed` (* (`CharacterMovementComponent.MaxWalkSpeed` _charactermovement) 2.0) _charactermovement)
  (`|AIMoveTo` null (`KismetMathLibrary.MakeVector` (.x (+ _returnvalue (* (`KismetMathLibrary.GetForwardVector` (`KismetMathLibrary.FindLookAtRotation` _returnvalue (`self.K2_GetActorLocation` _asbp_third_person_character))) -500.0))) (.y (+ _returnvalue (* (`KismetMathLibrary.GetForwardVector` (`KismetMathLibrary.FindLookAtRotation` _returnvalue (`self.K2_GetActorLocation` _asbp_third_person_character))) -500.0))) (.z _returnvalue)) null))

(event `NPCIdle_Event`
  (`KismetSystemLibrary.Delay` (`KismetMathLibrary.RandomFloatInRange` 0.0 5.0)))

(event `MoveToRandomLocation_Event`
  (`|AIMoveTo` null (`NavigationSystemV1.K2_GetRandomReachablePointInRadius` (`self.K2_GetActorLocation`) (`self.Radius`) null null) null (`self.AcceptanceRadius`)))

(event `self.AIPerception.OnTargetPerceptionUpdated`
  (params (Actor :type "Actor Object Reference") (Stimulus :type "AIStimulus Structure"))
  (`self.HandleSenses` Stimulus Actor))

(fn `HandleSenses`
  (params (Stimulus :type "AIStimulus Structure") (Actor :type "Actor Object Reference"))
  (bind (_age _expirationage _strength _stimuluslocation _receiverlocation _tag _bsuccessfullysensed) (break `AIStimulus` Stimulus))
  (bind (_age_2 _expirationage_2 _strength_2 _stimuluslocation_2 _receiverlocation_2 _tag_2) (break `AIStimulus` Stimulus))
  (bind _npc (`self.NPC`))
  (bind _npc_2 (`self.NPC`))
  (if (`|EnumInequality` (`/Game/Blueprints/BP_NPC.CurrentNPCState` (`self.NPC`)) "NewEnumerator3")
    (bind _returnvalue (`AIPerceptionSystem.GetSenseClassForStimulus` Stimulus))
    (if (== _returnvalue "/Script/AIModule.AISense_Sight")
      (if (`self.ActorHasTag` Actor "Player")
        (bind _output_get (set `/Game/Blueprints/BP_NPC.TargetActor` (`KismetMathLibrary.SelectObject` (`GameplayStatics.GetPlayerCharacter` 0) null _bsuccessfullysensed) (`self.NPC`)))
        (if _bsuccessfullysensed
          (bind _asbp_third_person_character (cast `/Game/Blueprints/BP_ThirdPersonCharacter` _output_get))
          (if (`/Game/Blueprints/BP_ThirdPersonCharacter.Notorious` _asbp_third_person_character)
            (`/Game/Blueprints/BP_NPC.Set NPCScared` _npc_2 true)
            (set `/Game/Blueprints/BP_NPC.CurrentNPCState` "NewEnumerator2" _npc_2)
            (`NavMovementComponent.StopActiveMovement` (`Character.CharacterMovement` _npc_2))))
        (else
          (return)))
      (elif (== _returnvalue "/Script/AIModule.AISense_Hearing")
        (if (or (== _tag_2 "NotoriousChitter") (== _tag_2 "Gun"))
          (`/Game/Blueprints/BP_NPC.Set NPCScared` _npc true)
          (if (`|EnumInequality` (`/Game/Blueprints/BP_NPC.CurrentNPCState` _npc) "NewEnumerator2")
            (set `/Game/Blueprints/BP_NPC.CurrentNPCState` "NewEnumerator2" _npc)
            (`NavMovementComponent.StopActiveMovement` (`Character.CharacterMovement` _npc)))
          (else
            (return)))
        (else
          (return))))))

(fn `UserConstructionScript`)