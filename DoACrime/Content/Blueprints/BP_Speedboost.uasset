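; BP_Speedboost is a coffee pickup that grants the player a speed boost on overlap.
; When a Player-tagged actor overlaps it, it casts player 0's character to BP_ThirdPersonCharacter and checks whether a boost is already running.
; If not, it triggers the character's SpeedBoostEvent, plays a pickup sound and destroys itself.
; Otherwise it stays and plays a "full" sound; both sounds get slight random volume and pitch variation.
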(event `self.ReceiveActorBeginOverlap`
  (params (OtherActor :type "Actor Object Reference"))
  (if (`self.ActorHasTag` OtherActor "Player")
    (bind _asbp_third_person_character (cast `/Game/Blueprints/BP_ThirdPersonCharacter` (`GameplayStatics.GetPlayerCharacter` 0)))
    (if (`/Game/Blueprints/BP_ThirdPersonCharacter.SpeedBoosting` _asbp_third_person_character)
      (`GameplayStatics.PlaySound2D` "/Game/Audio/SW_CoffeeFullSound.SW_CoffeeFullSound" (`KismetMathLibrary.RandomFloatInRange` 0.9 1.1) (`KismetMathLibrary.RandomFloatInRange` 0.9 1.1) 0.0 null null false)
      (else
        (`/Game/Blueprints/BP_ThirdPersonCharacter.SpeedBoost_Event` _asbp_third_person_character)
        (`GameplayStatics.PlaySound2D` "/Game/Audio/SW_PickUpCoffeeSound.SW_PickUpCoffeeSound" (`KismetMathLibrary.RandomFloatInRange` 0.9 1.1) (`KismetMathLibrary.RandomFloatInRange` 0.9 1.1) 0.0 null null false)
        (`self.K2_DestroyActor`)))))

(fn `UserConstructionScript`)