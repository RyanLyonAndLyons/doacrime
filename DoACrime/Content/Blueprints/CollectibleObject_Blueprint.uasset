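; Collectible pickup actor that advances tasks and the Noreity meter when a Player-tagged actor overlaps it.
; The construction script uses the collectible type to pick the mesh and Noreity value, with valuables worth more than food.
; On overlap it updates a general task plus a food or valuables task through the game mode's task list widget.
; It then adds its scaled value to the meter, plays a random-pitch sound, spawns pickup VFX and destroys itself.
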(event `self.ReceiveActorBeginOverlap`
  (params (OtherActor :type "Actor Object Reference"))
  (`parent.ReceiveActorBeginOverlap` OtherActor)
  (if (`self.ActorHasTag` OtherActor "Player")
    (bind _asbp_third_person_game_mode (cast `/Game/Blueprints/BP_ThirdPersonGameMode` (`GameplayStatics.GetGameMode`)))
    (`/Game/Blueprints/TaskListWidget.UpdateTask` (`/Game/Blueprints/BP_ThirdPersonGameMode.TaskListWidget` _asbp_third_person_game_mode) "NewEnumerator0")
    (switch `/Game/Blueprints/CollectibleObjectType` (`self.CollectibleObjectType`)
      (:`NewEnumerator2`
        (bind _tasklistwidget (`/Game/Blueprints/BP_ThirdPersonGameMode.TaskListWidget` _asbp_third_person_game_mode))
        (`/Game/Blueprints/TaskListWidget.UpdateTask` _tasklistwidget "NewEnumerator6" :!label _label))
      (:`NewEnumerator3`
        (`/Game/Blueprints/TaskListWidget.UpdateTask` _tasklistwidget "NewEnumerator2" :!label _label_2))
      (:`NewEnumerator4`
        (goto _label_2))
      (:`NewEnumerator5`
        (goto _label))
      (:`NewEnumerator6`
        (goto _label_2))
      (:`NewEnumerator7`
        (goto _label))
      (:`NewEnumerator16`
        (goto _label))
      (:`NewEnumerator17`
        (goto _label_2))
      (:`NewEnumerator18`
        (goto _label_2))
      (:`NewEnumerator19`
        (goto _label_2)))
    (`self.Collect Object`)))

(fn `Collect Object`
  (bind _asbp_third_person_game_mode (cast `/Game/Blueprints/BP_ThirdPersonGameMode` (`GameplayStatics.GetGameMode`)))
  (`/Game/Blueprints/NoreityMeter.UpdateNoreityMeter` (`/Game/Blueprints/BP_ThirdPersonGameMode.NoreityMeter` _asbp_third_person_game_mode) (/ (`self.NoreityValue`) 100.0))
  (`GameplayStatics.PlaySound2D` "/Game/Audio/SW_ItemGet.SW_ItemGet" 1.0 (`KismetMathLibrary.RandomFloatInRange` 0.5 1.5) 0.0 null null)
  (`NiagaraFunctionLibrary.SpawnSystemAtLocation` "/Game/VFX/NS_PickUp.NS_PickUp" (`SceneComponent.K2_GetComponentLocation` (`self.StaticMeshComponent`)))
  (`self.K2_DestroyActor`))

(fn `UserConstructionScript`
  (`parent.UserConstructionScript`)
  (`StaticMeshComponent.SetStaticMesh` (`self.StaticMeshComponent`) (select `/Game/Blueprints/CollectibleObjectType` (`self.CollectibleObjectType`) :`NewEnumerator2` "/Game/Assets/StaticMesh/SM_GoldBar.SM_GoldBar" :`NewEnumerator3` "/Game/Assets/StaticMesh/SM_Lollipop_002.SM_Lollipop_002" :`NewEnumerator4` "/Game/Assets/StaticMesh/SM_Lollipop_002.SM_Lollipop_002" :`NewEnumerator5` "/Game/Assets/StaticMesh/SM_MoneyStack.SM_MoneyStack" :`NewEnumerator6` "/Game/Assets/StaticMesh/SM_GranolaBar.SM_GranolaBar" :`NewEnumerator7` "/Game/Assets/StaticMesh/SM_Cellphone.SM_Cellphone" :`NewEnumerator16` "/Game/Assets/StaticMesh/SM_Coin.SM_Coin" :`NewEnumerator17` "/Game/Assets/StaticMesh/SM_Hotdog.SM_Hotdog" :`NewEnumerator18` "/Game/Assets/StaticMesh/SM_IceCream.SM_IceCream" :`NewEnumerator19` "/Game/Assets/StaticMesh/SM_Banana.SM_Banana" :!type "StaticMesh Object Reference"))
  (switch `/Game/Blueprints/CollectibleObjectType` (`self.CollectibleObjectType`)
    (:`NewEnumerator2`
      (set `self.NoreityValue` 5.0))
    (:`NewEnumerator3`
      (set `self.NoreityValue` 0.25 :!label _label))
    (:`NewEnumerator4`
      (goto _label))
    (:`NewEnumerator5`
      (set `self.NoreityValue` 3.0 :!label _label_2))
    (:`NewEnumerator6`
      (goto _label))
    (:`NewEnumerator7`
      (goto _label_2))
    (:`NewEnumerator16`
      (set `self.NoreityValue` 1.0))
    (:`NewEnumerator17`
      (goto _label))
    (:`NewEnumerator18`
      (goto _label))
    (:`NewEnumerator19`
      (goto _label))))